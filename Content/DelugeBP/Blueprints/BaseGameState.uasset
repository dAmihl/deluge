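; Base game state that exposes map lifecycle and messaging events, relaying them to the BaseGameMode.
; It caches the game mode on BeginPlay, then forwards server messages to it and, on authority only, map completion.
; It also stores the map's enemy spawn points.
; StartMap and OnActorDied are stubs containing only an authority switch.
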(event `self.ReceiveBeginPlay`
  (`self.SetupGameModeRef`))

(event `self.ReceiveTick`
  (params (DeltaSeconds :type "Float (single-precision)")))

(event `SetEnemySpawnPointsInMap`
  (params (spawnPoints :type "Array of /Game/DelugeBP/Blueprints/Misc/BaseEnemySpawn Object Reference"))
  (set `self.EnemySpawnPoints` spawnPoints))

(event `ServerMessage`
  (params (message :type String) (duration :type "Float (double-precision)"))
  (`/Game/DelugeBP/Blueprints/GameModes/BaseGameMode.ServerMessage` (`self.GameModeRef`) message duration))

(event `OnMapComplete`
  (`/Engine/EditorBlueprintResources/ActorMacros.Switch Has Authority`
    (:`Authority`
      (`/Game/DelugeBP/Blueprints/GameModes/BaseGameMode.MapCompleted` (`self.GameModeRef`)))))

(event `StartMap`
  (`/Engine/EditorBlueprintResources/ActorMacros.Switch Has Authority`))

(event `OnActorDied`
  (params (ActorDied :type "Actor Object Reference"))
  (`/Engine/EditorBlueprintResources/ActorMacros.Switch Has Authority`))

(fn `SetupGameModeRef`
  (bind _asbase_game_mode (cast `/Game/DelugeBP/Blueprints/GameModes/BaseGameMode` (`GameplayStatics.GetGameMode`)))
  (set `self.GameModeRef` _asbase_game_mode))

(fn `UserConstructionScript`)