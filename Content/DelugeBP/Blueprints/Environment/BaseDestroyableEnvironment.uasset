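; Base Blueprint for destructible environment actors that track health and report to the game mode when it runs out.
; GetDamage forwards to ReceiveDamage, which subtracts health only with authority.
; At zero or below, it passes itself to BaseGameMode's ActorDestroyed rather than destroying itself.
; The DestroyedActor event is left empty here.
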(event `self.ReceiveBeginPlay`)

(event `self.ReceiveActorBeginOverlap`
  (params (OtherActor :type "Actor Object Reference")))

(event `self.ReceiveTick`
  (params (DeltaSeconds :type "Float (single-precision)")))

(event `/Game/DelugeBP/Blueprints/Misc/IDestroyable.DestroyedActor`)

(event `ReceiveDamage`
  (params (damage :type "Float (double-precision)"))
  (`/Engine/EditorBlueprintResources/ActorMacros.Switch Has Authority`
    (:`Authority`
      (bind _output_get (set `self.Health` (- (`self.Health`) damage)))
      (if (<= _output_get 0.0)
        (bind _asbase_game_mode (cast `/Game/DelugeBP/Blueprints/GameModes/BaseGameMode` (`GameplayStatics.GetGameMode`)))
        (`/Game/DelugeBP/Blueprints/GameModes/BaseGameMode.ActorDestroyed` _asbase_game_mode self)))))

(event `/Game/DelugeBP/Blueprints/Misc/IDestroyable.GetDamage`
  (params (damageAmount :type "Float (single-precision)"))
  (`self.ReceiveDamage` damageAmount))

(fn `UserConstructionScript`
  (`parent.UserConstructionScript`))