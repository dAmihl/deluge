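; Base game mode for a multiplayer game, handling player registration, respawning, map travel and combat rules.
; Post-login registers controllers on the authority, feeding server message broadcasts; respawn replaces the pawn at a player start.
; Helpers validate hits via character vulnerability, log damage and deaths, and check whether all players occupy a trigger.
; Map completion sets the flag gating exit, while exit events are empty stubs and travel runs through a console command.
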(event EventBeginPlay
  (Development|PrintString "HELLO FROM THE RUSKI SIDE!!!"))

(event EventTick
  (params (DeltaSeconds :type Float%20%28single-precision%29)))

(event Custom|ServerMessage
  (params (message :type String) (duration :type Float%20%28single-precision%29))
  (for _array_element (Variables|Default|GetInGamePlayers)
    (Default|OnServerMessage _array_element message duration)))

(event Custom|ServerTravel
  (params (mapName :type String))
  (Networking|SwitchHasAuthority
    (:Authority
      (CallFunction|SrvStartTravel mapName))))

(event Custom|srvStartTravel
  (params (map%20name :type String))
  (Development|ExecuteConsoleCommand (Utilities|String|Append "ServerTravel " map%20name)))

(event Custom|ExitTriggerNotifier
  (params (actorsOnTrigger :type Array%20of%20Actor%20Object%20References)))

(event Custom|RegisterPlayerController
  (params (PlayerController :type Player%20Controller%20Object%20Reference))
  (CallFunction|AddPlayerController PlayerController))

(event Custom|RespawnPlayer
  (params (playerController :type Base%20Player%20Controller%20Object%20Reference) (character%20class :type Pawn%20Class%20Reference) (old%20pawn :type Pawn%20Object%20Reference))
  ;[1 1 1] Spawns a player
  (Networking|SwitchHasAuthority
    (:Authority
      (Pawn|UnPossess playerController)
      (Actor|DestroyActor old%20pawn)
      (bind _returnvalue (Game|SpawnActorfromClass character%20class (Transformation|GetActorTransform (Class|GameMode|FindPlayerStart playerController)) "AdjustIfPossibleButAlwaysSpawn" 0 0))
      (Pawn|Possess playerController _returnvalue)
      (Default|OnSpawn playerController)
      (bind _asbase_player_character (Utilities|Casting|CastToBasePlayerCharacter _returnvalue))
      (Variables|/Game/DelugeBP/Blueprints/Characters/Player/BasePlayerCharacter.BasePlayerCharacter_C|SetCurrentPlayerController _asbase_player_character playerController))))

(event EventPostLogin
  (params (NewPlayer :type Player%20Controller%20Object%20Reference))
  (CallFunction|RegisterPlayerController NewPlayer))

(event Custom|ExitMap)

(event Custom|CheckExitReady)

(event Custom|MapCompleted
  (Variables|Default|SetbIsMapCompleted true))

(fn ConstructionScript)

(fn ValidateActorHitsActor
  (params (fromActor :type Actor%20Object%20Reference) (toActor :type Actor%20Object%20Reference) (hitLocation :type Vector))
  (bind _asbase_character (Utilities|Casting|CastToBaseCharacter toActor)
    (:then
      (return (Variables|/Game/DelugeBP/Blueprints/Characters/BaseCharacter.BaseCharacter_C|GetbVulnerable _asbase_character)))
    (:CastFailed
      (return true))))

(fn ActorGivesDamagetoActor
  (params (fromActor :type Actor%20Object%20Reference) (toActor :type Actor%20Object%20Reference) (damage :type Float%20%28single-precision%29))
  (CallFunction|BattleLog (Utilities|String|Append (Utilities|GetDisplayName fromActor) " gives Damage  " (Utilities|String|ToString(Float) damage) " to " (Utilities|GetDisplayName toActor)))
  (return true))

(fn BattleLog
  (params (text :type String))
  (Development|PrintString text true true "(R=0.573312,G=0.000000,B=1.000000,A=1.000000)" 5.0))

(fn ActorDestroyed
  (params (deadActor :type Actor%20Object%20Reference))
  (CallFunction|BattleLog (Utilities|String|Append (Utilities|GetDisplayName deadActor) " died!!")))

(fn CheckAllPlayersinArray
  (params (actorArray :type Array%20of%20Actor%20Object%20References))
  (bind _numberplayersinarray (LocalVariables|GetnumberPlayersInArray))
  (for _array_element actorArray
    (bind _asbase_character (Utilities|Casting|CastToBaseCharacter _array_element))
    (bind _asbase_player_controller (Utilities|Casting|CastToBasePlayerController (Pawn|GetController _asbase_character)))
    (if (Utilities|Array|ContainsItem (Variables|/Script/Engine.GameState|GetPlayerArray (Game|GetGameState)) (Variables|/Script/Engine.Controller|GetPlayerState _asbase_player_controller))
      (Math|Integer|IncrementInt (LocalVariables|GetnumberPlayersInArray))))
  (Development|PrintString (Utilities|String|Append "Players on trigger: " (Utilities|String|ToString(Integer) _numberplayersinarray)))
  (return (== _numberplayersinarray (Utilities|Array|Length (Variables|/Script/Engine.GameState|GetPlayerArray (Game|GetGameState))))))

(fn CanExitMap
  (return (Variables|Default|GetbIsMapCompleted)))

(fn ActorIsPlayer
  (params (Actor :type Actor%20Object%20Reference))
  (Utilities|Casting|CastToBasePlayerCharacter Actor
    (:then
      (return true))
    (:CastFailed
      (return false))))

(fn GetRegisteredPlayers
  (return (Variables|Default|GetInGamePlayers)))

(fn AddPlayerController
  (params (PlayerController :type Player%20Controller%20Object%20Reference))
  (Networking|SwitchHasAuthority
    (:Authority
      (bind _asbase_player_controller (Utilities|Casting|CastToBasePlayerController PlayerController))
      (Utilities|Array|AddUnique (Variables|Default|GetInGamePlayers) _asbase_player_controller)
      (Default|ClientPostLogin _asbase_player_controller)
      (Development|PrintString "Player connected!")
      (Development|PrintString (Utilities|String|ToString(Integer) (Utilities|Array|Length (Variables|Default|GetInGamePlayers)))))))