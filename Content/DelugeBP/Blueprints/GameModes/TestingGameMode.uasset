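; TestingGameMode is a game mode that layers damage and destruction messaging onto its parent's combat rules.
; Hit validation passes only when the parent approves and the target implements the IDestroyable interface.
; After the parent handles damage or destruction, it sends GetDamageMessage to the damaged actor or DestroyedActorMessage to the dead one.
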(event `self.ReceiveBeginPlay`)

(event `self.ReceiveTick`
  (params (DeltaSeconds :type "Float (single-precision)")))

(event `self.ActorDestroyed`
  (params (deadActor :type "Actor Object Reference"))
  (`parent.ActorDestroyed` deadActor)
  (message `/Game/DelugeBP/Blueprints/Misc/IDestroyable.DestroyedActor` deadActor))

(fn `ActorGivesDamageToActor`
  (params (fromActor :type "Actor Object Reference") (toActor :type "Actor Object Reference") (damage :type "Float (double-precision)"))
  (returns (accepted :type Boolean))
  (bind _accepted (`parent.ActorGivesDamageToActor` fromActor toActor damage))
  (message `/Game/DelugeBP/Blueprints/Misc/IDestroyable.GetDamage` toActor damage)
  (return _accepted))

(fn `UserConstructionScript`
  (`parent.UserConstructionScript`))

(fn `ValidateActorHitsActor`
  (params (fromActor :type "Actor Object Reference") (toActor :type "Actor Object Reference") (hitLocation :type "Vector Structure"))
  (returns (accepted :type Boolean))
  (bind _accepted (`parent.ValidateActorHitsActor` fromActor toActor hitLocation))
  (return (and _accepted (`KismetSystemLibrary.DoesImplementInterface` toActor "/Game/DelugeBP/Blueprints/Misc/IDestroyable.IDestroyable_C"))))