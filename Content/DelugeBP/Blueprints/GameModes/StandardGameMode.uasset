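; StandardGameMode sets map rules for hits, damage, destruction and the group exit back to the Hub, extending its parent's logic.
; Hits count only on IDestroyable targets, and damage and destruction are relayed to the affected actors as messages.
; Exit trigger updates start a timer when all players stand on it and the parent check passes, otherwise pausing it; expiry server-travels to Hub.
; BeginPlay immediately marks the map completed.
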(event `self.ReceiveBeginPlay`
  (set `self.bIsMapCompleted` true))

(event `self.ReceiveTick`
  (params (DeltaSeconds :type "Float (single-precision)")))

(event `self.ActorDestroyed`
  (params (deadActor :type "Actor Object Reference"))
  (`parent.ActorDestroyed` deadActor)
  (message `/Game/DelugeBP/Blueprints/Misc/IDestroyable.DestroyedActor` deadActor))

(event `self.ExitTriggerNotifier`
  (params (actorsOnTrigger :type "Array of Actor Object Reference (by ref)"))
  (bind _allplayersinarray (`self.CheckAllPlayersInArray` actorsOnTrigger))
  (set `self.AllPlayersOnExit` _allplayersinarray)
  (`self.CheckExitReady`))

(event `self.CheckExitReady`
  (bind _canexit (`self.CanExitMap`))
  (if _canexit
    (`self.StartExit`)
    (else
      (`self.StopExit`))))

(event `StartExit`
  (`KismetSystemLibrary.PrintString` "Exit Started!")
  (bind _returnvalue (`KismetSystemLibrary.K2_SetTimerDelegate` (delegate `TimerExitFinished`) (`self.ExitMapTime`))))

(event `TimerExitFinished`
  (`self.ExitMap`))

(event `StopExit`
  (if (`KismetSystemLibrary.K2_IsValidTimerHandle` (stale `StartExit` _returnvalue))
    (`KismetSystemLibrary.PrintString` "Exit Stopped!")
    (`KismetSystemLibrary.K2_PauseTimerHandle` (stale `StartExit` _returnvalue))))

(event `self.ExitMap`
  (`self.ServerTravel` "Hub"))

(fn `ActorGivesDamageToActor`
  (params (fromActor :type "Actor Object Reference") (toActor :type "Actor Object Reference") (damage :type "Float (double-precision)"))
  (returns (accepted :type Boolean))
  (bind _accepted (`parent.ActorGivesDamageToActor` fromActor toActor damage))
  (message `/Game/DelugeBP/Blueprints/Misc/IDestroyable.GetDamage` toActor damage)
  (return _accepted))

(fn `CanExitMap`
  (returns (canExit :type Boolean))
  (bind _canexit (`parent.CanExitMap`))
  (return (and _canexit (`self.AllPlayersOnExit`))))

(fn `UserConstructionScript`
  (`parent.UserConstructionScript`))

(fn `ValidateActorHitsActor`
  (params (fromActor :type "Actor Object Reference") (toActor :type "Actor Object Reference") (hitLocation :type "Vector Structure"))
  (returns (accepted :type Boolean))
  (bind _accepted (`parent.ValidateActorHitsActor` fromActor toActor hitLocation))
  (return (and _accepted (`KismetSystemLibrary.DoesImplementInterface` toActor "/Game/DelugeBP/Blueprints/Misc/IDestroyable.IDestroyable_C"))))