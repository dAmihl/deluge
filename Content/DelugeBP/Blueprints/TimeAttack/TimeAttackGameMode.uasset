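; Game mode for Time Attack that handles actor deaths and decides which hits are valid.
; When an AI actor dies, it is unpossessed and destroyed after a despawn timer, while a player death is only logged.
; Hit validation extends the parent check with an XOR on player status, so hits count only between a player and a non-player.
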(event `self.ReceiveTick`
  (params (DeltaSeconds :type "Float (single-precision)"))
  (`parent.ReceiveTick` 0.0))

(event `self.ActorDestroyed`
  (params (deadActor :type "Actor Object Reference"))
  (`parent.ActorDestroyed` deadActor)
  (bind _isplayer (`self.ActorIsPlayer` deadActor))
  (if _isplayer
    (`self.BattleLog` "PLAYER DIED!!!!")
    (else
      (bind _returnvalue (`AIBlueprintHelperLibrary.GetAIController` deadActor))
      (`/Engine/EditorBlueprintResources/StandardMacros.IsValid` _returnvalue
        (:`Is Valid`
          (`Controller.UnPossess` _returnvalue)
          (`KismetSystemLibrary.K2_SetTimerDelegate` (delegate `DespawnActor`) (`self.DespawnTime`)))))))

(event `DespawnActor`
  (`self.K2_DestroyActor` (stale `self.ActorDestroyed` deadActor)))

(event `self.RegisterPlayerController`
  (params (PlayerController :type "PlayerController Object Reference"))
  (`parent.RegisterPlayerController` PlayerController)
  (`KismetSystemLibrary.PrintString` "TIME ATTACK"))

(fn `UserConstructionScript`
  (`parent.UserConstructionScript`))

(fn `ValidateActorHitsActor`
  (params (fromActor :type "Actor Object Reference") (toActor :type "Actor Object Reference") (hitLocation :type "Vector Structure"))
  (returns (accepted :type Boolean))
  (bind _accepted (`parent.ValidateActorHitsActor` fromActor toActor hitLocation))
  (bind _isplayer (`self.ActorIsPlayer` fromActor))
  (bind _isplayer_2 (`self.ActorIsPlayer` toActor))
  (return (and _accepted (xor _isplayer _isplayer_2))))