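; Game state for Time Attack mode that runs a timed enemy wave and detects when the map is complete.
; On authority, timers from the game mode's settings spawn random enemy classes at random points, each targeting a random player, until time runs out.
; Spawned enemies are tracked until death.
; Tick checks for timer expiry with none left, then notifies the game mode and announces completion once.
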(event `self.ReceiveBeginPlay`
  (`parent.ReceiveBeginPlay`)
  (`self.StartMap`))

(event `self.ReceiveTick`
  (params (DeltaSeconds :type "Float (single-precision)"))
  (`self.CheckMapComplete`))

(event `self.SetupGameModeRef`
  (`parent.SetupGameModeRef`)
  (bind _astime_attack_game_mode (cast `/Game/DelugeBP/Blueprints/TimeAttack/TimeAttackGameMode` (`self.GameModeRef`)))
  (set `self.TimeAttackGameModeRef` _astime_attack_game_mode))

(event `self.OnMapComplete`
  (`/Game/DelugeBP/Blueprints/GameModes/BaseGameMode.MapCompleted` (`self.TimeAttackGameModeRef`))
  (`self.ServerMessage` "MAP COMPLETE!" 2.0))

(event `CheckMapComplete`
  (bind _iscomplete (`self.IsMapComplete`))
  (if _iscomplete
    (`/Engine/EditorBlueprintResources/StandardMacros.DoOnce` false
      (:`Completed`
        (`self.OnMapComplete`)))))

(event `self.OnActorDied`
  (params (ActorDied :type "Actor Object Reference"))
  (`parent.OnActorDied` ActorDied)
  (bind _asbase_enemy_character (cast `/Game/DelugeBP/Blueprints/Characters/Enemy/BaseEnemyCharacter` ActorDied))
  (`KismetArrayLibrary.Array_RemoveItem` (`self.spawnedEnemies`) _asbase_enemy_character))

(event `self.StartMap`
  (`self.StartTimeAttackTimer`)
  (`self.StartSpawnTimer`)
  (`self.ServerMessage` "MAP STARTED!" 2.0))

(event `StartTimeAttackTimer`
  ;[1 1 1] Starts the match timer
  (`/Engine/EditorBlueprintResources/ActorMacros.Switch Has Authority`
    (:`Authority`
      (`KismetSystemLibrary.K2_SetTimerDelegate` (delegate `TimerHandle`) (`/Game/DelugeBP/Blueprints/TimeAttack/TimeAttackGameMode.TimeAttackTime` (`self.TimeAttackGameModeRef`))))))

(event `TimerHandle`
  ;[1 1 1] Starts the match timer
  (set `self.timerRunOut` true)
  (`KismetSystemLibrary.K2_PauseTimerHandle` (`self.SpawnTimer`)))

(event `StartSpawnTimer`
  ;[1 1 1] Starts the spawn timer with gamemodes spawn rate
  (`/Engine/EditorBlueprintResources/ActorMacros.Switch Has Authority`
    (:`Authority`
      (bind _returnvalue (`KismetSystemLibrary.K2_SetTimerDelegate` (delegate `SpawnTimerHandle`) (`/Game/DelugeBP/Blueprints/TimeAttack/TimeAttackGameMode.SpawnRate` (`self.TimeAttackGameModeRef`)) true))
      (set `self.SpawnTimer` _returnvalue))))

(event `SpawnTimerHandle`
  ;[1 1 1] Starts the spawn timer with gamemodes spawn rate
  (`self.SpawnEnemy`))

(event `SpawnEnemy`
  (bind _enemyspawnpoints (`self.EnemySpawnPoints`))
  (bind _enemyclasses (`self.EnemyClasses`))
  ;[1 1 1] Spawns enemy of random class at random spawn point
  (bind _returnvalue (`|SpawnActorFromClass` (`KismetArrayLibrary.Array_Get` _enemyclasses (`KismetMathLibrary.RandomIntegerInRange` 0 (- (`KismetArrayLibrary.Array_Length` _enemyclasses) 1))) (`KismetMathLibrary.MakeTransform` (`SceneComponent.K2_GetComponentLocation` (`/Game/DelugeBP/Blueprints/Misc/BaseEnemySpawn.DefaultSceneRoot` (`KismetArrayLibrary.Array_Get` _enemyspawnpoints (`KismetMathLibrary.RandomIntegerInRange` 0 (- (`KismetArrayLibrary.Array_Length` _enemyspawnpoints) 1)))))) "Undefined" "OverrideRootScale"))
  (`self.GiveEnemyRandomTarget` _returnvalue)
  (`KismetArrayLibrary.Array_AddUnique` (`self.spawnedEnemies`) _returnvalue))

(event `GiveEnemyRandomTarget`
  (params (enemy :type "/Game/DelugeBP/Blueprints/Characters/Enemy/BaseEnemyCharacter Object Reference"))
  ;[1 1 1] Gives the AI a random player as target
  (`/Engine/EditorBlueprintResources/ActorMacros.Switch Has Authority`
    (:`Authority`
      (bind _returnvalue (`AIBlueprintHelperLibrary.GetAIController` enemy))
      (bind _asbase_aicontroller (cast `/Game/DelugeBP/Blueprints/Characters/Enemy/BaseAIController` _returnvalue))
      (bind _outactors (`GameplayStatics.GetAllActorsOfClass` "/Game/DelugeBP/Blueprints/Characters/Player/BasePlayerCharacter.BasePlayerCharacter_C"))
      (`/Game/DelugeBP/Blueprints/Characters/Enemy/BaseAIController.SetCharacterTarget` _asbase_aicontroller (`KismetArrayLibrary.Array_Get` _outactors (`KismetMathLibrary.RandomIntegerInRange` 0 (- (`KismetArrayLibrary.Array_Length` _outactors) 1)))))))

(fn `IsMapComplete`
  (returns (isComplete :type Boolean))
  (return (and (`self.timerRunOut`) (== (`KismetArrayLibrary.Array_Length` (`self.spawnedEnemies`)) 0))))

(fn `UserConstructionScript`
  (`parent.UserConstructionScript`))