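; BaseSaveGame is a save game object that stores a player's character attributes and character data.
; SavePlayerData copies both structs from the PlayerController's attributes and character data components into the save, and LoadPlayerDataInController writes them back.
; It only transfers values in memory, with no slot reads or writes, and InitCleanSaveGame is an empty function.
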(event `SavePlayerData`
  (params (`player Controller` :type "/Game/DelugeBP/Blueprints/Characters/Player/PlayerController/BasePlayerController Object Reference"))
  (set `self.baseAttributesStruct` (`/Game/DelugeBP/Blueprints/Characters/Components/Attributes/BaseAttributesComponent.CharacterAttributes` (`/Game/DelugeBP/Blueprints/Characters/Player/PlayerController/BasePlayerController.PlayerAttributesComponent` `player Controller`)))
  (set `self.characterDataStruct` (`/Game/DelugeBP/Blueprints/Characters/Components/CharacterData/PlayerCharacterDataComponent.dataStruct` (`/Game/DelugeBP/Blueprints/Characters/Player/PlayerController/BasePlayerController.PlayerCharacterDataComponent` `player Controller`))))

(event `LoadPlayerDataInController`
  (params (`player controller` :type "/Game/DelugeBP/Blueprints/Characters/Player/PlayerController/BasePlayerController Object Reference"))
  (set `/Game/DelugeBP/Blueprints/Characters/Components/Attributes/BaseAttributesComponent.CharacterAttributes` (`self.baseAttributesStruct`) (`/Game/DelugeBP/Blueprints/Characters/Player/PlayerController/BasePlayerController.PlayerAttributesComponent` `player controller`))
  (set `/Game/DelugeBP/Blueprints/Characters/Components/CharacterData/PlayerCharacterDataComponent.dataStruct` (`self.characterDataStruct`) (`/Game/DelugeBP/Blueprints/Characters/Player/PlayerController/BasePlayerController.PlayerCharacterDataComponent` `player controller`)))

(fn `InitCleanSaveGame`)