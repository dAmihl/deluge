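; Base player character Blueprint that handles the cosmetic side of weapons: first-person gun mesh, fire montage and sound, muzzle flash and hit effects.
; The gun attaches to Mesh2P's grip socket and takes its mesh from the controller's equipped weapon class.
; A RepNotify on the action state starts or stops the muzzle emitter, attached to the first-person gun for the local player and the third-person gun otherwise.
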(event `self.ReceiveBeginPlay`)

(event `self.ReceiveTick`
  (params (DeltaSeconds :type "Float (single-precision)")))

(event `/Game/DelugeBP/Blueprints/Misc/IHasHitEffects.SpawnHitFX`
  (params (location :type "Vector Structure"))
  (`GameplayStatics.SpawnEmitterAtLocation` (`self.HitFXEmitterClass`) location))

(fn `GetWeaponPosition`
  (returns (vecPosition :type "Vector Structure"))
  (return (`SceneComponent.K2_GetComponentLocation` (`self.FP_Gun`))))

(fn `OnRep_CurrentPlayerActionState`
  (switch `/Game/DelugeBP/Blueprints/Player/PlayerActionState` (`self.CurrentPlayerActionState`)
    (:`NewEnumerator0`
      (`self.StopAttackFX`))
    (:`NewEnumerator1`
      (`self.StartAttackFX`))))

(fn `PlayLocalFireWeaponAnimation`
  (`AnimInstance.Montage_Play` (`SkeletalMeshComponent.GetAnimInstance` (`self.Mesh2P`)) "/Game/DelugeAssets/Animations/FirstPersonFire_Montage.FirstPersonFire_Montage" 1.0)
  (`GameplayStatics.PlaySoundAtLocation` "/Game/DelugeAssets/Audio/FirstPersonTemplateWeaponFire02.FirstPersonTemplateWeaponFire02"))

(fn `SetWeaponMesh`
  (bind _asbase_player_controller (cast `/Game/DelugeBP/Blueprints/Player/BasePlayerController` (`self.GetController`)))
  (bind _output_get (set `self.CurrentPlayerController` _asbase_player_controller))
  (`SkinnedMeshComponent.SetSkinnedAssetAndUpdate` (`self.FP_Gun`) (`.WeaponMesh_2_D1487BB04D3B2A0B4DF9CC86A1A6B79D` (break `/Game/DelugeBP/Blueprints/Weapon/SWeapon_Base` (defaults `/Game/DelugeBP/Blueprints/Player/BasePlayerCharacter` (`/Game/DelugeBP/Blueprints/Player/BasePlayerController.CurrentlyEquippedWeapon` _output_get))))))

(fn `StartAttackFX`
  (`self.isLocalCharacter`
    (:`True`
      (bind _returnvalue (`GameplayStatics.SpawnEmitterAttached` "/Game/Effects/ParticleSystems/Weapons/AssaultRifle/Muzzle/P_AssaultRifle_MF.P_AssaultRifle_MF" (`self.FP_Gun`) (`KismetStringLibrary.Conv_StringToName` (`self.WeaponMuzzleFXBoneName`))))
      (set `self.AttackFXRef` _returnvalue))
    (:`False`
      (bind _returnvalue_2 (`GameplayStatics.SpawnEmitterAttached` "/Game/Effects/ParticleSystems/Weapons/AssaultRifle/Muzzle/P_AssaultRifle_MF.P_AssaultRifle_MF" (`self.TP_Gun`) (`KismetStringLibrary.Conv_StringToName` (`self.WeaponMuzzleFXBoneName`))))
      (set `self.AttackFXRef` _returnvalue_2))))

(fn `StartReloadFX`)

(fn `StopAttackFX`
  (bind _attackfxref (`self.AttackFXRef`))
  (`/Engine/EditorBlueprintResources/StandardMacros.IsValid` _attackfxref
    (:`Is Valid`
      (`ActorComponent.K2_DestroyComponent` _attackfxref))))

(fn `UserConstructionScript`
  (`SceneComponent.K2_AttachTo` (`self.FP_Gun`) (`self.Mesh2P`) "GripPoint" "SnapToTargetIncludingScale" true))